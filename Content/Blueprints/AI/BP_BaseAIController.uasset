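; BP_BaseAIController is an enemy AI controller that runs the BT_Enemy behavior tree when it possesses a pawn.
; Its AI perception updates are filtered to the first player character and written to the blackboard.
; The Player key holds that character while sensed and is cleared otherwise, while Location records the stimulus position on every such update.
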(event OnTargetPerceptionUpdated(AIPerception)
  (params (Actor :type Actor%20Object%20Reference) (Stimulus :type AI%20Stimulus%20Structure))
  (bind (_age _expirationage _strength _stimuluslocation _receiverlocation _tag _bsuccessfullysensed) (Utilities|Struct|BreakAIStimulus Stimulus))
  (bind _returnvalue (Game|GetPlayerCharacter 0))
  ;[0.15 0.15 0.15 0.5] Set player when AI see him
  (if (== Actor _returnvalue)
    (AI|Components|Blackboard|SetValueasObject (Variables|Default|GetBlackboard) (Utilities|Name|MakeLiteralName "Player") (select _bsuccessfullysensed _returnvalue 0))
    (AI|Components|Blackboard|SetValueasVector (Variables|Default|GetBlackboard) (Utilities|Name|MakeLiteralName "Location") _stimuluslocation)))

(event EventPossess
  (params (PossessedPawn :type Pawn%20Object%20Reference))
  ;[0.15 0.15 0.15 0.5] Run BT
  (AI|RunBehaviorTree "/Game/Blueprints/AI/BT_Enemy.BT_Enemy"))

(fn ConstructionScript)