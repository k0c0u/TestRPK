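; BP_Gate is a world gate actor that swings two parts open when activated.
; It starts closed with ticking disabled, and Activate enables tick, which plays a timeline while the gate is not open.
; The timeline alpha lerps the yaw of two scene components from opposite starting angles to a shared open angle.
; On finish it sets IsOpen, with no closing logic and tick left enabled.
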(event EventBeginPlay
  (Actor|Tick|SetActorTickEnabled false)
  (Variables|Default|SetIsOpen false))

(event EventTick
  (params (DeltaSeconds :type Float%20%28single-precision%29))
  (if (not (Variables|Default|GetIsOpen))
    (bind _alpha (Timeline|Timeline Play)
      (:Update
        (Utilities|FlowControl|Sequence
          (:then_0
            (Transformation|SetRelativeRotation (Variables|Default|GetScene1) (Math|Rotator|MakeRotator 0.0 0.0 (Math|Float|Lerp 0.0 -9e+01 _alpha)) false false))
          (:then_1
            (Transformation|SetRelativeRotation (Variables|Default|GetScene2) (Math|Rotator|MakeRotator 0.0 0.0 (Math|Float|Lerp -179.0 -9e+01 _alpha)) false false))))
      (:Finished
        (Variables|Default|SetIsOpen true)))))

(event EventActivate
  (Actor|Tick|SetActorTickEnabled true))

(fn ConstructionScript)