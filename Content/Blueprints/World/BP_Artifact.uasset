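; BP_Artifact is an interactable world artifact that rises or shifts to an offset location and spins once activated.
; Tick is off from BeginPlay, which caches the end location, until Interact enables it.
; Tick moves the actor at constant speed while IsActorInEndLocation, which is true when not yet arrived, and keeps yawing it indefinitely.
; GetArtifactNameAndDescription exposes its text and whether both fields are filled.
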(event EventBeginPlay
  ;[0.15 0.15 0.15 0.5] Of tick and Set end location
  (Actor|Tick|SetActorTickEnabled false)
  (CallFunction|SetEndLocation))

(event EventTick
  (params (DeltaSeconds :type Float%20%28single-precision%29))
  ;[0.15 0.15 0.15 0.5] Change location and Rotation
  (Utilities|FlowControl|Sequence
    (:then_0
      (CallFunction|UpdateLocation DeltaSeconds))
    (:then_1
      (Class|Actor|AddActorWorldRotation (Math|Rotator|MakeRotator 0.0 0.0 (Variables|Default|GetRotateYawSpeed))))))

(event EventInteract
  ;[0.15 0.15 0.15 0.5] Activate Artifact
  (Actor|Tick|SetActorTickEnabled true))

(fn ConstructionScript)

(fn SetEndLocation
  (Variables|Default|SetEndLocation (+ (Transformation|GetActorLocation) (Variables|Default|GetLocationAfterInteract))))

(fn IsActorinEndLocation
  (return (Utilities|Operators|NotEqual(!=) (Transformation|GetActorLocation) (Variables|Default|GetEndLocation) 0.1)))

(fn UpdateLocation
  (params (DeltaTime :type Float%20%28single-precision%29))
  (if (CallFunction|IsActorinEndLocation)
    (Transformation|SetActorLocation (Math|Interpolation|VInterptoConstant (Transformation|GetActorLocation) (Variables|Default|GetEndLocation) DeltaTime (Variables|Default|GetInterpSpeed)) false false)
    (else
      (return))))

(fn GetArtifactNameandDescription
  (return (Variables|Default|GetName) (Variables|Default|GetDescription) (and (not (Utilities|Array|IsEmpty (Variables|Default|GetName))) (not (Utilities|Array|IsEmpty (Variables|Default|GetDescription))))))