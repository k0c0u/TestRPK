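; BP_Trap is a world trap that damages any BP_BaseCharacter overlapping its Box.
; Any overlap also recolors the trap through a dynamic material instance created at BeginPlay, with no reset to the original color.
; A WBP_Indicator viewport widget follows the trap on screen, re-centered every Tick by projecting its offset world location for player 0.
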(event OnComponentBeginOverlap(Box)
  (params (OverlappedComponent :type Primitive%20Component%20Object%20Reference) (OtherActor :type Actor%20Object%20Reference) (OtherComp :type Primitive%20Component%20Object%20Reference) (OtherBodyIndex :type Integer) (bFromSweep :type Boolean) (SweepResult :type Hit%20Result%20Structure%20%28by%20ref%29))
  ;[0.15 0.15 0.15 0.5] Apply damage
  (CallFunction|ApplyDamage OtherActor)
  ;[0.15 0.15 0.15 0.5] Set new color for trap
  (CallFunction|SetNewTrapColor))

(event EventBeginPlay
  ;[0.15 0.15 0.15 0.5] Create indicator widget
  (CallFunction|CreateIndicatorWidget)
  ;[0.15 0.15 0.15 0.5] Create dynamic material
  (CallFunction|CreateDynamicMaterial))

(event EventTick
  (params (DeltaSeconds :type Float%20%28single-precision%29))
  ;[0.15 0.15 0.15 0.5] Update indicator widget position
  (CallFunction|UpdateWidgetPosition))

(fn ConstructionScript)

(fn SetNewTrapColor
  (bind _dynamicmaterial (Variables|Default|GetDynamicMaterial))
  (Utilities|IsValid _dynamicmaterial
    (:Is%20Valid
      (bind _returnvalue (Rendering|Material|GetVectorParameterValue _dynamicmaterial (Variables|Default|GetMaterial%20Parameter%20Name) :!class /Script/Engine.MaterialInstanceDynamic))
      (if (!= _returnvalue (Variables|Default|GetNewColor))
        (Rendering|Material|SetVectorParameterValue _dynamicmaterial (Variables|Default|GetMaterial%20Parameter%20Name) (Variables|Default|GetNewColor) :!class /Script/Engine.MaterialInstanceDynamic)))))

(fn CreateIndicatorWidget
  (bind _returnvalue (UserInterface|CreateWidget "/Game/UI/WBP_Indicator.WBP_Indicator_C" (Game|GetPlayerController 0)))
  (bind _output_get (Variables|Default|SetIndicatorRef _returnvalue))
  (UserInterface|Viewport|AddtoViewport _output_get 0))

(fn CreateDynamicMaterial
  (bind _staticmesh (Variables|Default|GetStaticMesh))
  (bind _returnvalue (Rendering|Material|CreateDynamicMaterialInstance _staticmesh 0 (Rendering|Material|GetMaterial _staticmesh 0) "None" :!class /Script/Engine.PrimitiveComponent))
  (Variables|Default|SetDynamicMaterial _returnvalue))

(fn ApplyDamage
  (params (InputPin :type Actor%20Object%20Reference))
  (if (Class|GameplayStatics|ObjectIsA InputPin "/Game/Blueprints/Core/BP_BaseCharacter.BP_BaseCharacter_C")
    (Game|Damage|ApplyDamage InputPin (Variables|Default|GetBase%20Damage) 0 self "/Script/Engine.DamageType")))

(fn UpdateWidgetPosition
  (bind _returnvalue (Game|GetPlayerController 0))
  (bind _returnvalue_2 (Transformation|GetActorLocation))
  (bind _positionoffset (Variables|Default|GetPositionOffset))
  (bind _returnvalue_3 (+ _returnvalue_2 _positionoffset))
  (bind (_screenposition _returnvalue_4) (Class|WidgetLayoutLibrary|ProjectWorldLocationtoWidgetPosition _returnvalue _returnvalue_3 true))
  (if _returnvalue_4
    (Class|UserWidget|SetPositioninViewport (Variables|Default|GetIndicatorRef) (- _screenposition (/ (Class|Widget|GetDesiredSize (Variables|Default|GetIndicatorRef)) 2.0)) false)))