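; BP_Lever is an interactable lever that rotates to an end position and activates a linked actor.
; Interact enables Tick and immediately sends ActivateMessage to ControlledActor, printing an error if it is invalid or lacks InteractInterface.
; Tick rotates the Scene component toward EndRotation at constant speed, then switches itself off.
; Despite its name, IsEndLeverRotation returns true while the lever has yet to reach EndRotation.
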(event EventBeginPlay
  (Actor|Tick|SetActorTickEnabled false))

(event EventTick
  (params (DeltaSeconds :type Float%20%28single-precision%29))
  (CallFunction|UpdateLeverRotation DeltaSeconds)
  (if (not (CallFunction|IsEndLeverRotation))
    (Actor|Tick|SetActorTickEnabled false)))

(event EventInteract
  (bind _controlledactor (Variables|Default|GetControlledActor))
  (Actor|Tick|SetActorTickEnabled true)
  (Utilities|IsValid _controlledactor
    (:Is%20Valid
      (if (Utilities|DoesObjectImplementInterface _controlledactor "/Script/TestRPK.InteractInterface")
        (Class|InteractInterface|Activate(Message) _controlledactor)
        (else
          (Development|PrintString "BP_Lever::Interact ControlledActor not implement interface"))))
    (:Is%20Not%20Valid
      (Development|PrintString "BP_Lever::Interact ControlledActor not valid"))))

(fn ConstructionScript)

(fn IsEndLeverRotation
  (return (Utilities|Operators|NotEqual(!=) (Variables|/Script/Engine.SceneComponent|GetRelativeRotation (Variables|Default|GetScene)) (Variables|Default|GetEndRotation) 0.1)))

(fn UpdateLeverRotation
  (params (DeltaTime :type Float%20%28single-precision%29))
  (if (CallFunction|IsEndLeverRotation)
    (Transformation|SetRelativeRotation (Variables|Default|GetScene) (Class|KismetMathLibrary|RInterptoConstant (Variables|/Script/Engine.SceneComponent|GetRelativeRotation (Variables|Default|GetScene)) (Variables|Default|GetEndRotation) DeltaTime (Variables|Default|GetInterp%20Speed)) false false)
    (else
      (return))))